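; BP_Rope provides functions to link two actors with a visual cable or a physics constraint.
; ConnectCable spawns a CableActor at the first actor, snaps it on, and attaches the cable's end to the second actor with a fixed length.
; ConnectPhysicsConstrained separately binds both actors' StaticMeshComponents through its constraint component.
; The event graph and construction script are empty, so both functions rely on external callers.
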(event EventBeginPlay)

(event Collision|EventActorBeginOverlap
  (params (OtherActor :type Actor%20Object%20Reference)))

(event EventTick
  (params (DeltaSeconds :type Float%20%28single-precision%29)))

(fn ConstructionScript)

(fn ConnectCable
  (params (FirstActor :type Actor%20Object%20Reference) (SecondActor :type Actor%20Object%20Reference))
  (bind _returnvalue (Game|SpawnActorfromClass "/Script/CableComponent.CableActor" (Math|Conversions|ToTransform(Vector) (Transformation|GetActorLocation FirstActor)) "Undefined" 0 0))
  (Transformation|AttachActorToActor _returnvalue FirstActor "None" "SnapToTarget" "KeepRelative" "KeepRelative" true)
  (Class|CableComponent|SetAttachEndto (Variables|/Script/CableComponent.CableActor|GetCableComponent _returnvalue) SecondActor "None" "None")
  (Variables|/Script/CableComponent.CableComponent|SetEndLocation (Variables|/Script/CableComponent.CableActor|GetCableComponent _returnvalue) "0, 0, 0")
  (Variables|/Script/CableComponent.CableComponent|SetCableLength (Variables|/Script/CableComponent.CableActor|GetCableComponent _returnvalue) 2.5e+02))

(fn ConnectPhysicsConstrained
  (params (FirstActor :type Actor%20Object%20Reference) (SecondActor :type Actor%20Object%20Reference))
  (Class|PhysicsConstraintComponent|SetConstrainedComponents (Variables|Default|GetConstraintComp) (Actor|GetComponentbyClass FirstActor "/Script/Engine.StaticMeshComponent") "None" (Actor|GetComponentbyClass SecondActor "/Script/Engine.StaticMeshComponent") "None"))