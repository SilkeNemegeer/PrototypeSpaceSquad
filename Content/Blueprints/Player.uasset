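; Player pawn with physics-driven jetpack movement, a grappling hook and the ability to rope astronauts into a chain.
; Tick turns movement input and held fly flags into mesh impulses, and roll flags into local rotation.
; Grapple input traces from the camera, then Tick interpolates the cable to the hit and impulses the player toward it.
; A forward trace finds "Astronaut"-tagged actors, which interact input links via BP_Rope to the player or last chained astronaut.
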(event Custom|FlyUp
  (bind _mesh (Variables|Default|GetMesh))
  (bind _returnvalue (Transformation|GetWorldRotation _mesh))
  ;[1 1 1] Fly Up and down
  (Physics|AddImpulse (Variables|Default|GetMesh) (* (Math|Vector|GetUpVector (Math|Rotator|MakeRotator (.roll _returnvalue) (.pitch _returnvalue) (.yaw _returnvalue))) (Variables|Default|Getjetstrength)) "None" false))

(event Custom|Descend
  (bind _mesh (Variables|Default|GetMesh))
  (bind _returnvalue (Transformation|GetWorldRotation _mesh))
  ;[1 1 1] Fly Up and down
  (Physics|AddImpulse (Variables|Default|GetMesh) (* (* (Math|Vector|GetUpVector (Math|Rotator|MakeRotator (.roll _returnvalue) (.pitch _returnvalue) (.yaw _returnvalue))) (Variables|Default|Getjetstrength)) -1.0) "None" false))

(event Custom|RollLeft
  ;[1 1 1] Roll left right
  (Transformation|AddActorLocalRotation (Math|Rotator|MakeRotator (* (* (Utilities|Time|GetWorldDeltaSeconds) (Variables|Default|GetrollSpeed)) -1.0) 0.0 0.0) false false))

(event Custom|RollRight
  ;[1 1 1] Roll left right
  (Transformation|AddActorLocalRotation (Math|Rotator|MakeRotator (* (Utilities|Time|GetWorldDeltaSeconds) (Variables|Default|GetrollSpeed)) 0.0 0.0) false false))

(event Custom|StopGrapple
  (bind _grappling_hook (Variables|Default|GetGrappling%20hook))
  (Variables|Default|SetisGrappling false)
  (Variables|Default|SetfinishedGrappling false)
  (Rendering|SetVisibility _grappling_hook false false)
  (Transformation|SetWorldLocation _grappling_hook "0, 0,50.000000" false false))

(event EventBeginPlay
  (bind _grappling_hook (Variables|Default|GetGrappling%20hook))
  ;[1 1 1] Set Grapple
  (Rendering|SetVisibility _grappling_hook false false)
  (Variables|/Script/CableComponent.CableComponent|SetCableLength _grappling_hook 0.0)
  (Variables|/Script/CableComponent.CableComponent|SetCableWidth _grappling_hook 8.0)
  (Variables|/Script/CableComponent.CableComponent|SetEndLocation _grappling_hook "0, 0, 0"))

(event Collision|EventActorBeginOverlap
  (params (OtherActor :type Actor%20Object%20Reference)))

(event EventTick
  (params (DeltaSeconds :type Float%20%28single-precision%29))
  (bind _returnvalue (Transformation|GetActorLocation))
  ;[1 1 1] Process movement jetpack
  (Utilities|FlowControl|Sequence
    (:then_0
      (bind _returnvalue_2 (Class|Pawn|ConsumeMovementInputVector))
      (Physics|AddImpulse (Variables|Default|GetMesh) (* (* _returnvalue_2 DeltaSeconds) (Variables|Default|Getspeed)) "None" true))
    (:then_1
      (if (Variables|Default|GetisFlyingUp)
        (CallFunction|FlyUp)
        (elif (Variables|Default|GetisFlyingDown)
          (CallFunction|Descend))))
    (:then_2
      (if (Variables|Default|GetisRollingLeft)
        (CallFunction|RollLeft)
        (elif (Variables|Default|GetisRollingRight)
          (CallFunction|RollRight))))
    (:then_3
      (if (Variables|Default|GetisGrappling)
        (if (Variables|Default|GetfinishedGrappling)
          (CallFunction|MovePlayertoGrapple)
          (Utilities|FlowControl|Delay 0.2)
          (CallFunction|StopGrapple)
          (else
            (bind _reachedend (CallFunction|ShootGrapple))
            (Variables|Default|SetfinishedGrappling _reachedend)))))
    (:then_4
      ;[1 1 1] Attach people
      (bind (_outhit _returnvalue_3) (Collision|LineTraceForObjects (+ _returnvalue "0, 0,80.000000") (+ _returnvalue (* (Transformation|GetActorForwardVector) 2.5e+02) "0,0,80.000000") (Utilities|Array|MakeArray "ObjectTypeQuery1" "ObjectTypeQuery2" "ObjectTypeQuery3" "ObjectTypeQuery4" "ObjectTypeQuery5" "ObjectTypeQuery6") false 0 "None"))
      (Utilities|IsValid (.HitActor (Collision|BreakHitResult _outhit))
        (:Is%20Valid
          (if _returnvalue_3
            (if (>= (Utilities|Array|Length (Variables|/Script/Engine.Actor|GetTags (.HitActor (Collision|BreakHitResult _outhit)))) 1)
              (for _array_element (Variables|/Script/Engine.Actor|GetTags (.HitActor (Collision|BreakHitResult _outhit)))
                (if (Utilities|Name|Equal(Name) _array_element "Astronaut")
                  (Development|PrintString "Found astronaut!!")
                  (Variables|Default|SetIsAstronautInRange true)
                  (Variables|Default|SetInteractableObject (.HitActor (Collision|BreakHitResult _outhit)))
                  (else
                    (Variables|Default|SetIsAstronautInRange false)
                    (Variables|Default|SetInteractableObject 0)))))))))))

(event Input|ActionEvents|InputActionShootGrapple
  (params (Key :type Key%20Structure :default "None"))
  (bind _returnvalue (Transformation|GetActorLocation))
  ;[1 1 1] Grapple input process
  (:Pressed
    (bind (_outhit _returnvalue_2) (Collision|LineTraceForObjects _returnvalue (+ _returnvalue (* (Math|Vector|GetForwardVector (Variables|Default|GetCamera)) (Variables|Default|GetgrappleRange))) (Utilities|Array|MakeArray "ObjectTypeQuery1" "ObjectTypeQuery2") false 0 "None"))
    (if _returnvalue_2
      (Variables|Default|SetisGrappling true)
      (Variables|Default|SetgrappleEndLocation (.Location (Collision|BreakHitResult _outhit)))
      (else
        (CallFunction|StopGrapple)))))

(event Input|ActionEvents|InputActionAttachPeople
  (params (Key :type Key%20Structure :default "None"))
  (bind _self self)
  (bind _interactableobject (Variables|Default|GetInteractableObject))
  (bind _interactableobject_2 (Variables|Default|GetInteractableObject))
  (bind _chainedastronauts (Variables|Default|GetChainedAstronauts))
  (bind _returnvalue (Utilities|Array|LastIndex _chainedastronauts))
  (bind _output (Utilities|Array|Get(acopy) _chainedastronauts _returnvalue))
  ;[1 1 1] Attach people
  (:Pressed
    (if (Variables|Default|GetIsAstronautInRange)
      (Utilities|IsValid (Variables|Default|GetInteractableObject)
        (:Is%20Valid
          (if (== (Utilities|Array|Length (Variables|Default|GetChainedAstronauts)) 0)
            (bind _returnvalue_2 (Game|SpawnActorfromClass "/Game/Blueprints/BP_Rope.BP_Rope_C" (Math|Transform|MakeTransform "0, 0, 0") "Undefined" 0 0))
            (Transformation|AttachActorToActor _returnvalue_2 self "None" "SnapToTarget" "KeepRelative" "KeepRelative" true)
            (Utilities|Array|Add (Variables|Default|GetChainedAstronauts) _interactableobject_2)
            (Default|ConnectCable _returnvalue_2 _self _interactableobject_2)
            (Default|ConnectPhysicsConstrained _returnvalue_2 _self _interactableobject_2)
            (else
              (bind _returnvalue_3 (Game|SpawnActorfromClass "/Game/Blueprints/BP_Rope.BP_Rope_C" (Math|Transform|MakeTransform "0, 0, 0") "Undefined" 0 0))
              (Transformation|AttachActorToActor _returnvalue_3 _output "None" "SnapToTarget" "KeepRelative" "KeepRelative" true)
              (Default|ConnectCable _returnvalue_3 _output _interactableobject)
              (Default|ConnectPhysicsConstrained _returnvalue_3 _output _interactableobject)
              (Utilities|Array|Add (Variables|Default|GetChainedAstronauts) _interactableobject))))))))

(event Input|ActionEvents|InputActionRollLeft
  (params (Key :type Key%20Structure :default "None"))
  ;[1 1 1] Roll left right
  (:Pressed
    (Variables|Default|SetisRollingLeft true))
  (:Released
    (Variables|Default|SetisRollingLeft false)))

(event Input|ActionEvents|InputActionRollRight
  (params (Key :type Key%20Structure :default "None"))
  ;[1 1 1] Roll left right
  (:Pressed
    (Variables|Default|SetisRollingRight true))
  (:Released
    (Variables|Default|SetisRollingRight false)))

(event Input|ActionEvents|InputActionFlyUp
  (params (Key :type Key%20Structure :default "None"))
  ;[1 1 1] Fly Up and down
  (:Pressed
    (Variables|Default|SetisFlyingUp true))
  (:Released
    (Variables|Default|SetisFlyingUp false)))

(event Input|ActionEvents|InputActionFlyDown
  (params (Key :type Key%20Structure :default "None"))
  ;[1 1 1] Fly Up and down
  (:Pressed
    (Variables|Default|SetisFlyingDown true))
  (:Released
    (Variables|Default|SetisFlyingDown false)))

(event Input|KeyboardEvents|F
  (params (Key :type Key%20Structure :default "None"))
  (bind _self self)
  (bind _interactableobject (Variables|Default|GetInteractableObject))
  (bind _interactableobject_2 (Variables|Default|GetInteractableObject))
  (bind _chainedastronauts (Variables|Default|GetChainedAstronauts))
  (bind _returnvalue (Utilities|Array|LastIndex _chainedastronauts))
  (bind _output (Utilities|Array|Get(acopy) _chainedastronauts _returnvalue))
  ;[1 1 1] Attach people
  (:Pressed
    (if (Variables|Default|GetIsAstronautInRange)
      (Utilities|IsValid (Variables|Default|GetInteractableObject)
        (:Is%20Valid
          (if (== (Utilities|Array|Length (Variables|Default|GetChainedAstronauts)) 0)
            (bind _returnvalue_2 (Game|SpawnActorfromClass "/Game/Blueprints/BP_Rope.BP_Rope_C" (Math|Transform|MakeTransform "0, 0, 0") "Undefined" 0 0))
            (Transformation|AttachActorToActor _returnvalue_2 self "None" "SnapToTarget" "KeepRelative" "KeepRelative" true)
            (Utilities|Array|Add (Variables|Default|GetChainedAstronauts) _interactableobject_2)
            (Default|ConnectCable _returnvalue_2 _self _interactableobject_2)
            (Default|ConnectPhysicsConstrained _returnvalue_2 _self _interactableobject_2)
            (else
              (bind _returnvalue_3 (Game|SpawnActorfromClass "/Game/Blueprints/BP_Rope.BP_Rope_C" (Math|Transform|MakeTransform "0, 0, 0") "Undefined" 0 0))
              (Transformation|AttachActorToActor _returnvalue_3 _output "None" "SnapToTarget" "KeepRelative" "KeepRelative" true)
              (Default|ConnectCable _returnvalue_3 _output _interactableobject)
              (Default|ConnectPhysicsConstrained _returnvalue_3 _output _interactableobject)
              (Utilities|Array|Add (Variables|Default|GetChainedAstronauts) _interactableobject))))))))

(fn ConstructionScript)

(fn ShootGrapple
  (bind _grappling_hook (Variables|Default|GetGrappling%20hook))
  (bind _grappleendlocation (Variables|Default|GetgrappleEndLocation))
  (bind _returnvalue (Transformation|GetWorldLocation _grappling_hook))
  (Rendering|SetVisibility _grappling_hook true false)
  (if (<= (Math|Vector|VectorLength (- _returnvalue _grappleendlocation)) 1e+02)
    (return true)
    (else
      (Transformation|SetWorldLocation _grappling_hook (Math|Interpolation|VInterpTo _returnvalue _grappleendlocation (Utilities|Time|GetWorldDeltaSeconds) 2e+01) false false)
      (return false))))

(fn MovePlayertoGrapple
  (Physics|AddImpulse (Variables|Default|GetMesh) (* (- (Variables|Default|GetgrappleEndLocation) (Transformation|GetActorLocation)) (* (Variables|Default|GetgrapplingSpeed) (Utilities|Time|GetWorldDeltaSeconds))) "None" true))

(fn RetrieveGrapple
  (bind _grappling_hook (Variables|Default|GetGrappling%20hook))
  (Transformation|SetWorldLocation _grappling_hook (Math|Interpolation|VInterpTo (Transformation|GetWorldLocation _grappling_hook) (Variables|Default|GetgrappleEndLocation) (Utilities|Time|GetWorldDeltaSeconds) 5e+02) false false))