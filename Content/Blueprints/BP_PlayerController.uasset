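; Player controller Blueprint that turns movement and look axis inputs into motion on the controlled pawn.
; Move axes add movement input along the pawn's forward and right vectors, taken from its full actor rotation.
; Look axes apply local pitch and yaw directly to the pawn, scaled by LookSpeed and delta time with pitch negated, rather than driving control rotation.
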(event EventBeginPlay)

(event EventTick
  (params (DeltaSeconds :type Float%20%28single-precision%29)))

(event Input|AxisEvents|InputAxisMoveForward
  (params (AxisValue :type Float%20%28single-precision%29))
  (bind _returnvalue (Pawn|GetControlledPawn))
  (bind _returnvalue_2 (Transformation|GetActorRotation _returnvalue))
  ;[1 1 1] Left joystick control
  (Pawn|Input|AddMovementInput _returnvalue (Math|Vector|GetForwardVector (Math|Rotator|MakeRotator (.roll _returnvalue_2) (.pitch _returnvalue_2) (.yaw _returnvalue_2))) AxisValue false))

(event Input|AxisEvents|InputAxisMoveRight
  (params (AxisValue :type Float%20%28single-precision%29))
  (bind _returnvalue (Pawn|GetControlledPawn))
  (bind _returnvalue_2 (Transformation|GetActorRotation _returnvalue))
  ;[1 1 1] Left joystick control
  (Pawn|Input|AddMovementInput _returnvalue (Math|Vector|GetRightVector (Math|Rotator|MakeRotator (.roll _returnvalue_2) (.pitch _returnvalue_2) (.yaw _returnvalue_2))) AxisValue false))

(event Input|AxisEvents|InputAxisLookRight
  (params (AxisValue :type Float%20%28single-precision%29))
  ;[1 1 1] Look controls
  (Transformation|AddActorLocalRotation (Pawn|GetControlledPawn) (Math|Rotator|MakeRotator 0.0 0.0 (* (* (Utilities|Time|GetWorldDeltaSeconds) (Variables|Default|GetlookSpeed)) AxisValue)) false false))

(event Input|AxisEvents|InputAxisLookUp
  (params (AxisValue :type Float%20%28single-precision%29))
  ;[1 1 1] Look controls
  (Transformation|AddActorLocalRotation (Pawn|GetControlledPawn) (Math|Rotator|MakeRotator 0.0 (* (* (* (Utilities|Time|GetWorldDeltaSeconds) (Variables|Default|GetlookSpeed)) AxisValue) -1.0) 0.0) false false))

(fn ConstructionScript)